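; BP_PassThrough is a two-sided passage actor that tells overlapping actors they can walk through it from one end to the other.
; Entering the Pass1 or Pass2 trigger sends the actor InteractPass with this blueprint, plus WalkThrough with start and end taken from Location1 and Location2.
; Each side reverses the start and end points and sets the Leftright flag oppositely.
; Leaving either trigger resends both messages with an empty reference and zero locations.
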(event `self.pass1.OnComponentBeginOverlap`
  (params (OverlappedComponent :type "PrimitiveComponent Object Reference") (OtherActor :type "Actor Object Reference") (OtherComp :type "PrimitiveComponent Object Reference") (OtherBodyIndex :type Integer) (bFromSweep :type Boolean) (SweepResult :type "HitResult Structure (by ref)"))
  (message `/Game/BP/BPI_Character.interactPass` OtherActor self)
  (message `/Game/BP/BPI_Character.walkThrough` OtherActor (`SceneComponent.K2_GetComponentLocation` (`self.location1`)) (`SceneComponent.K2_GetComponentLocation` (`self.location2`)) true))

(event `self.pass1.OnComponentEndOverlap`
  (params (OverlappedComponent :type "PrimitiveComponent Object Reference") (OtherActor :type "Actor Object Reference") (OtherComp :type "PrimitiveComponent Object Reference") (OtherBodyIndex :type Integer))
  (message `/Game/BP/BPI_Character.interactPass` OtherActor null)
  (message `/Game/BP/BPI_Character.walkThrough` OtherActor (0.0 0.0 0.0) (0.0 0.0 0.0) true))

(event `self.pass2.OnComponentBeginOverlap`
  (params (OverlappedComponent :type "PrimitiveComponent Object Reference") (OtherActor :type "Actor Object Reference") (OtherComp :type "PrimitiveComponent Object Reference") (OtherBodyIndex :type Integer) (bFromSweep :type Boolean) (SweepResult :type "HitResult Structure (by ref)"))
  (message `/Game/BP/BPI_Character.interactPass` OtherActor self)
  (message `/Game/BP/BPI_Character.walkThrough` OtherActor (`SceneComponent.K2_GetComponentLocation` (`self.location2`)) (`SceneComponent.K2_GetComponentLocation` (`self.location1`)) false))

(event `self.pass2.OnComponentEndOverlap`
  (params (OverlappedComponent :type "PrimitiveComponent Object Reference") (OtherActor :type "Actor Object Reference") (OtherComp :type "PrimitiveComponent Object Reference") (OtherBodyIndex :type Integer))
  (message `/Game/BP/BPI_Character.interactPass` OtherActor null)
  (message `/Game/BP/BPI_Character.walkThrough` OtherActor (0.0 0.0 0.0) (0.0 0.0 0.0) false))

(fn `UserConstructionScript`)