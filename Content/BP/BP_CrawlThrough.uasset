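; Crawl-through passage actor that offers a traversal route between two end points to any actor entering either end.
; Each end has a collision box that, on overlap, passes the passage reference and start/end world locations to that actor through message calls, swapping direction per end.
; Leaving either box resends the interact message without a reference.
; The passage only supplies data, leaving the movement itself to the receiving actor.
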(event `self.boxCollPoint1.OnComponentBeginOverlap`
  (params (OverlappedComponent :type "PrimitiveComponent Object Reference") (OtherActor :type "Actor Object Reference") (OtherComp :type "PrimitiveComponent Object Reference") (OtherBodyIndex :type Integer) (bFromSweep :type Boolean) (SweepResult :type "HitResult Structure (by ref)"))
  (message `/Game/BP/BPI_Character.interactTunnel ` OtherActor self)
  (message `/Game/BP/BPI_Character.walkThrough` OtherActor (`SceneComponent.K2_GetComponentLocation` (`self.point1`)) (`SceneComponent.K2_GetComponentLocation` (`self.point2`)) true))

(event `self.boxCollPoint1.OnComponentEndOverlap`
  (params (OverlappedComponent :type "PrimitiveComponent Object Reference") (OtherActor :type "Actor Object Reference") (OtherComp :type "PrimitiveComponent Object Reference") (OtherBodyIndex :type Integer))
  (message `/Game/BP/BPI_Character.interactTunnel ` OtherActor null))

(event `self.boxCollPoint2.OnComponentBeginOverlap`
  (params (OverlappedComponent :type "PrimitiveComponent Object Reference") (OtherActor :type "Actor Object Reference") (OtherComp :type "PrimitiveComponent Object Reference") (OtherBodyIndex :type Integer) (bFromSweep :type Boolean) (SweepResult :type "HitResult Structure (by ref)"))
  (message `/Game/BP/BPI_Character.interactTunnel ` OtherActor self)
  (message `/Game/BP/BPI_Character.walkThrough` OtherActor (`SceneComponent.K2_GetComponentLocation` (`self.point2`)) (`SceneComponent.K2_GetComponentLocation` (`self.point1`)) true))

(event `self.boxCollPoint2.OnComponentEndOverlap`
  (params (OverlappedComponent :type "PrimitiveComponent Object Reference") (OtherActor :type "Actor Object Reference") (OtherComp :type "PrimitiveComponent Object Reference") (OtherBodyIndex :type Integer))
  (message `/Game/BP/BPI_Character.interactTunnel ` OtherActor null))

(fn `UserConstructionScript`)